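; Base NPC AI controller that runs BT_BaseNPC and steers it through blackboard keys.
; Sight perception tracks the player, with delayed forgetting, while Tick asks LevelControl about forbidden behavior and triggers dialogue, escalating by weight.
; Dialogue requests are prioritized by cause: forbidden, level control, then script, unless instant.
; Branch functions set patrol, wait or break states, record LastActivity for resuming, and can delay renewed reactions to the player.
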(event OnPerceptionUpdated(AIPerception)
  (params (UpdatedActors :type Array%20of%20Actor%20Object%20References))
  (bind _aiperception (Variables|Default|GetAIPerception))
  (bind _aiperception_2 (Variables|Default|GetAIPerception))
  (bind _outactors (Class|AIPerceptionComponent|GetPerceivedActors _aiperception_2 "/Script/AIModule.AISense_Sight"))
  (bind _outactors_2 (Class|AIPerceptionComponent|GetPerceivedActors _aiperception "/Script/AIModule.AISense_Sight"))
  ;[1 1 1] На каждый апдейт персепшена проверяем, есть ли игрок в поле зрения. Если есть, то записываем его в блекборд, если нет - очищаем его переменную в блекборде
  (if (Utilities|Array|IsValidIndex _outactors_2 (Utilities|Array|FindItem _outactors_2 (.Player (CallFunction|GetPlayer))))
    (Variables|Default|SetSeePlayerRightNow true)
    (Utilities|IsValid (CallFunction|GetBlackboardPlayer)
      (:Is%20Not%20Valid
        (CallFunction|SetBlackboardPlayer true)))
    (else
      (Utilities|IsValid (CallFunction|GetBlackboardPlayer)
        (:Is%20Valid
          (Variables|Default|SetSeePlayerRightNow false)
          (Utilities|FlowControl|RetriggerableDelay 5.0)
          (if (not (Utilities|Array|IsValidIndex _outactors (Utilities|Array|FindItem _outactors (.Player (CallFunction|GetPlayer)))))
            (CallFunction|SetBlackboardPlayer false)))))))

(event Custom|DelayCanReactToPlayer
  (params (Duration :type Float%20%28single-precision%29))
  (Utilities|FlowControl|Delay Duration)
  (Blackboard|BBSetCanReacttoPlayer true))

(event EventBeginPlay
  (bind _levelcontrol (CallFunction|GetLevelControl))
  (Variables|Default|SetLevelControl _levelcontrol))

(event EventTick
  (params (DeltaSeconds :type Float%20%28single-precision%29))
  (Development|PrintString (Utilities|String|ToString(Integer) (Variables|Default|GetCurrentForbiddenEventWeight)) true true "(R=0.000000,G=0.660000,B=1.000000,A=1.000000)" 0.0)
  (Development|PrintString (Utilities|GetDisplayName (AI|Components|Blackboard|GetValueasObject (AI|GetBlackboard 0) (Utilities|Name|MakeLiteralName "Player"))) true true "(R=0.000000,G=0.660000,B=1.000000,A=1.000000)" 0.0)
  (if (Variables|Default|GetSeePlayerRightNow)
    (if (ScalableFloat|GetValueasBool (AI|GetBlackboard self) (Utilities|Name|MakeLiteralName "CanReactToPlayer"))
      (Utilities|IsValid (AI|Components|Blackboard|GetValueasObject (AI|GetBlackboard self) (Utilities|Name|MakeLiteralName "Player"))
        (:Is%20Valid
          (bind (_foundforbidden _forbiddenaction _weight) (Default|ReacttoForbiddenBehavior (Variables|Default|GetLevelControl) (.AsBase%20NPC (Utilities|Casting|CastToBaseNPC (Pawn|GetControlledPawn self)))))
          (if _foundforbidden
            (if (ScalableFloat|GetValueasBool (AI|GetBlackboard 0) (Utilities|Name|MakeLiteralName "PlayerDoSomethingForbidden"))
              (if (> _weight (Variables|Default|GetCurrentForbiddenEventWeight))
                (Variables|Default|SetCurrentForbiddenEventWeight _weight :!label _label)
                (Blackboard|BBSetPlayerDoSomethingForbidden true)
                (Blackboard|BBSetLastSeeingForbiddenActivity _forbiddenaction)
                (Blackboard|BBSetWantActiononPlayer true)
                (Activity|StartDialogBranch false "None" false false false "NewEnumerator0"))
              (else
                (goto _label)))))))))

(event EventOnPossess
  (params (PossessedPawn :type Pawn%20Object%20Reference))
  (bind _output_get (Variables|Default|SetBaseNPC (.AsBase%20NPC (Utilities|Casting|CastToBaseNPC PossessedPawn))))
  (Blackboard|BBSetWaitingPoint (Variables|/Game/Blueprints/AI/BaseNPC.BaseNPC_C|GetWaitingPoint _output_get))
  (Blackboard|BBSetRotationPoint (Variables|/Game/Blueprints/AI/BaseNPC.BaseNPC_C|GetRotatePoint _output_get)))

(fn ConstructionScript
  (AI|RunBehaviorTree "/Game/Blueprints/AI/BT_BaseNPC.BT_BaseNPC"))

(fn GetBlackboardPlayer
  (return (AI|Components|Blackboard|GetValueasObject (AI|GetBlackboard 0) (Utilities|Name|MakeLiteralName "Player"))))

(fn SetBlackboardPlayer
  (params (Set :type Boolean))
  (if Set
    (AI|Components|Blackboard|SetValueasObject (AI|GetBlackboard 0) (Utilities|Name|MakeLiteralName "Player") (.Player (CallFunction|GetPlayer)))
    (else
      (AI|Components|Blackboard|SetValueasObject (AI|GetBlackboard 0) (Utilities|Name|MakeLiteralName "Player") 0))))

(fn GetPawn
  (return (.AsBase%20NPC (Utilities|Casting|CastToBaseNPC (Pawn|GetControlledPawn)))))

(fn BBSetNeedtoStartDialog
  (params (True :type Boolean))
  (AI|Components|Blackboard|SetValueasBool (AI|GetBlackboard 0) (Utilities|Name|MakeLiteralName "NeedToStartDialog") True))

(fn BBSetGoBetweenPoints
  (params (True :type Boolean))
  (AI|Components|Blackboard|SetValueasBool (AI|GetBlackboard 0) (Utilities|Name|MakeLiteralName "GoBetweenPoints") True))

(fn BBSetMoveBetweenPointsСonsistently
  (params (True :type Boolean))
  (AI|Components|Blackboard|SetValueasBool (AI|GetBlackboard 0) (Utilities|Name|MakeLiteralName "MoveBetweenPointsСonsistently") True))

(fn BBSetCurrentPointtoGo
  (params (CurrentPointToGo :type Object%20Object%20Reference))
  (AI|Components|Blackboard|SetValueasObject (AI|GetBlackboard 0) (Utilities|Name|MakeLiteralName "CurrentPointToGo") CurrentPointToGo))

(fn BBSetinRegularMode
  (params (True :type Boolean))
  (AI|Components|Blackboard|SetValueasBool (AI|GetBlackboard 0) (Utilities|Name|MakeLiteralName "InRegularMode") True))

(fn BBSetSearchingforPlayer
  (params (True :type Boolean))
  (AI|Components|Blackboard|SetValueasBool (AI|GetBlackboard 0) (Utilities|Name|MakeLiteralName "SearchingForPlayer") True))

(fn BBSetWantActiononPlayer
  (params (True :type Boolean))
  (AI|Components|Blackboard|SetValueasBool (AI|GetBlackboard 0) (Utilities|Name|MakeLiteralName "WantActionOnPlayer") True))

(fn BBSetWaitingPoint
  (params (WaitingPoint :type Object%20Object%20Reference))
  (AI|Components|Blackboard|SetValueasObject (AI|GetBlackboard 0) (Utilities|Name|MakeLiteralName "WaitingPoint") WaitingPoint))

(fn BBSetRotationPoint
  (params (RotatePoint :type Object%20Object%20Reference))
  (AI|Components|Blackboard|SetValueasObject (AI|GetBlackboard 0) (Utilities|Name|MakeLiteralName "RotatePoint") RotatePoint))

(fn BBSetWaitingTIme
  (params (WaitingTIme :type Float%20%28single-precision%29))
  (AI|Components|Blackboard|SetValueasFloat (AI|GetBlackboard 0) (Utilities|Name|MakeLiteralName "WaitingTIme") WaitingTIme))

(fn BBSetSearchinCertainPoints
  (params (True :type Boolean))
  (AI|Components|Blackboard|SetValueasBool (AI|GetBlackboard 0) (Utilities|Name|MakeLiteralName "SearchInCertainPoints") True))

(fn BBSetCertainSearchPoint
  (params (CertainSearchPoint :type Target%20Point%20Object%20Reference))
  (AI|Components|Blackboard|SetValueasObject (AI|GetBlackboard 0) (Utilities|Name|MakeLiteralName "CertainSearchPoint") CertainSearchPoint))

(fn BBSetCanReacttoPlayer
  (params (True :type Boolean))
  (AI|Components|Blackboard|SetValueasBool (AI|GetBlackboard 0) (Utilities|Name|MakeLiteralName "CanReactToPlayer") True))

(fn BBSetPlayerDoSomethingForbidden
  (params (True :type Boolean))
  (AI|Components|Blackboard|SetValueasBool (AI|GetBlackboard 0) (Utilities|Name|MakeLiteralName "PlayerDoSomethingForbidden") True))

(fn GoBetweenPointsBranch
  (params (WaitingTIme :type Float%20%28single-precision%29) (Randomly :type Boolean) (ReactToPlayerDelay :type Float%20%28single-precision%29))
  (Blackboard|BBSetWaitingTIme WaitingTIme)
  (if Randomly
    (Blackboard|BBSetGoBetweenPoints true)
    (Blackboard|BBSetMoveBetweenPointsСonsistently false)
    (Variables|/Game/Blueprints/AI/BaseNPC.BaseNPC_C|SetLastActivity (Variables|Default|GetBaseNPC) "NewEnumerator7")
    (else
      (Blackboard|BBSetGoBetweenPoints false)
      (Blackboard|BBSetMoveBetweenPointsСonsistently true)
      (Variables|/Game/Blueprints/AI/BaseNPC.BaseNPC_C|SetLastActivity (Variables|Default|GetBaseNPC) "NewEnumerator8")))
  (Blackboard|BBSetinRegularMode true)
  (Blackboard|BBSetWantActiononPlayer false)
  (Blackboard|BBSetPlayerDoSomethingForbidden false)
  (Blackboard|BBSetNeedtoWait false)
  (Blackboard|BBSetWantActiononPlayer false)
  (Blackboard|BBSetCanReacttoPlayer false)
  (CallFunction|DelayCanReacttoPlayer ReactToPlayerDelay))

(fn BBSetNeedtoWait
  (params (True :type Boolean))
  (AI|Components|Blackboard|SetValueasBool (AI|GetBlackboard 0) (Utilities|Name|MakeLiteralName "NeedToWait") True))

(fn MoveandWaitBranch
  (params (WaitingPoint :type Object%20Object%20Reference) (RotatePoint :type Object%20Object%20Reference) (ReactToPlayerDelay :type Float%20%28single-precision%29))
  (Utilities|IsValid WaitingPoint
    (:Is%20Valid
      (Blackboard|BBSetWaitingPoint WaitingPoint))
    (:Is%20Not%20Valid
      _))
  (Utilities|IsValid RotatePoint
    (:Is%20Valid
      (Blackboard|BBSetRotationPoint RotatePoint))
    (:Is%20Not%20Valid
      _))
  (Blackboard|BBSetNeedtoWait true)
  (Blackboard|BBSetinRegularMode true)
  (Blackboard|BBSetGoBetweenPoints false)
  (Blackboard|BBSetPlayerDoSomethingForbidden false)
  (Blackboard|BBSetWantActiononPlayer false)
  (Blackboard|BBSetCanReacttoPlayer false)
  (CallFunction|DelayCanReacttoPlayer ReactToPlayerDelay)
  (Variables|/Game/Blueprints/AI/BaseNPC.BaseNPC_C|SetLastActivity (Variables|Default|GetBaseNPC) "NewEnumerator9"))

(fn StartLastActivity
  (switch Utilities|FlowControl|Switch|SwitchonE_ActivityType (Variables|/Game/Blueprints/AI/BaseNPC.BaseNPC_C|GetLastActivity (Variables|Default|GetBaseNPC))
    (:NewEnumerator7
      (Activity|GoBetweenPointsBranch 2.0 true 5.0))
    (:NewEnumerator8
      (Activity|GoBetweenPointsBranch 2.0 false 5.0))
    (:NewEnumerator9
      (Activity|MoveandWaitBranch 0 0 5.0))
    (:NewEnumerator11
      (Activity|BreakBehaviorTree 5.0))
    (:NewEnumerator12
      ;[1 1 1] ВРЕМЕННАЯ ЗАГЛУШКА
      ; ЛИБО УБРАТЬ, ЛИБО ЗАМЕНИТЬ
      (Activity|BreakBehaviorTree 5.0))))

(fn StartDialogBranch
  (params (StartDialogInstantly :type Boolean) (StartedReplic :type Name) (StartDialogWithThisReplic :type Boolean) (IgnoreForbiddenBehavior :type Boolean) (SearchInCertainPoints :type Boolean) (Causer :type E_DialogStartCauser%20Enum :default "NewEnumerator3"))
  (if StartDialogWithThisReplic
    (Blackboard|BBSetStartDialogwithReplic true) ; Задаем конкретную реплику. Она НЕ БУДЕТ УЧИТЫВАТЬСЯ при запрещенном действии
    (Blackboard|BBSetStartDialogwithThisReplic StartedReplic))
  (LocalVariables|SetL_SearchInCertainPoints SearchInCertainPoints)
  (if StartDialogInstantly
    (Blackboard|BBDialogConditionSetter true true true (LocalVariables|GetL_SearchInCertainPoints))
    (Blackboard|BBMovingConditionSetter false false false false)
    (else
      (switch Utilities|FlowControl|Switch|SwitchonE_DialogStartCauser Causer
        (:NewEnumerator0
          (switch Utilities|FlowControl|Switch|SwitchonE_DialogStartCauser (Variables|Default|GetCurrentReasonForStartDialog)
            (:NewEnumerator3
              _)
            (:NewEnumerator1
              _)
            (:NewEnumerator2
              _))
          (Variables|Default|SetCurrentReasonForStartDialog "NewEnumerator0")
          (Blackboard|BBDialogConditionSetter false true true (LocalVariables|GetL_SearchInCertainPoints))
          (Blackboard|BBMovingConditionSetter false false false false))
        (:NewEnumerator1
          (switch Utilities|FlowControl|Switch|SwitchonE_DialogStartCauser (Variables|Default|GetCurrentReasonForStartDialog)
            (:NewEnumerator3
              (Variables|Default|SetCurrentReasonForStartDialog "NewEnumerator1"))
            (:NewEnumerator2
              (Variables|Default|SetCurrentReasonForStartDialog "NewEnumerator1")))
          (Blackboard|BBDialogConditionSetter false true true (LocalVariables|GetL_SearchInCertainPoints))
          (Blackboard|BBMovingConditionSetter false false false false))
        (:NewEnumerator2
          (switch Utilities|FlowControl|Switch|SwitchonE_DialogStartCauser (Variables|Default|GetCurrentReasonForStartDialog)
            (:NewEnumerator3
              (Variables|Default|SetCurrentReasonForStartDialog "NewEnumerator2")
              (Blackboard|BBDialogConditionSetter false true true (LocalVariables|GetL_SearchInCertainPoints))
              (Blackboard|BBMovingConditionSetter false false false false))))))))

(fn BBSetStartDialogInstantly
  (params (True :type Boolean))
  (AI|Components|Blackboard|SetValueasBool (AI|GetBlackboard 0) (Utilities|Name|MakeLiteralName "StartDialogInstantly") True))

(fn BBSetinDialog
  (params (True :type Boolean))
  (AI|Components|Blackboard|SetValueasBool (AI|GetBlackboard 0) (Utilities|Name|MakeLiteralName "InDialog") True))

(fn BBSetStartDialogwithReplic
  (params (True :type Boolean))
  (AI|Components|Blackboard|SetValueasBool (AI|GetBlackboard 0) (Utilities|Name|MakeLiteralName "StartDialogWithReplic") True))

(fn SetStartedDialoginLevelControl
  (Default|ChooseStartedReplicwithPlayer (Variables|Default|GetLevelControl) (Variables|Default|GetBaseNPC)))

(fn BreakBehaviorTree
  (params (ReactToPlayerDelay :type Float%20%28single-precision%29))
  (Variables|/Game/Blueprints/AI/BaseNPC.BaseNPC_C|SetLastActivity (Variables|Default|GetBaseNPC) "NewEnumerator11")
  (Blackboard|BBSetinRegularMode false)
  (Blackboard|BBSetinDialog false)
  (Blackboard|BBSetWantActiononPlayer false)
  (if (Variables|/Game/Blueprints/AI/BaseNPC.BaseNPC_C|GetNPCCanReactToPlayer (Variables|Default|GetBaseNPC))
    (Blackboard|BBSetCanReacttoPlayer false)
    (CallFunction|DelayCanReacttoPlayer ReactToPlayerDelay)
    (else
      (Blackboard|BBSetCanReacttoPlayer false))))

(fn SetStartedReplicifNotNull
  (params (StartedReplic :type Name))
  (if (not (Utilities|Name|Equal(Name) StartedReplic "None"))
    (Variables|/Game/Blueprints/AI/BaseNPC.BaseNPC_C|SetStartedReplic (Variables|Default|GetBaseNPC) StartedReplic)))

(fn BBSetIgnoreCheckifArrivetoPlayer
  (params (True :type Boolean))
  (AI|Components|Blackboard|SetValueasBool (AI|GetBlackboard 0) (Utilities|Name|MakeLiteralName "IgnoreCheckIfArriveToPlayer") True))

(fn BBSetLastSeeingForbiddenActivity
  (params (ForbiddenActivity :type String))
  (Class|BlackboardComponent|SetValueasString (AI|GetBlackboard 0) (Utilities|Name|MakeLiteralName "LastSeeingForbiddenActivity") ForbiddenActivity))

(fn BBDialogConditionSetter
  (params (StartDialogInstantly :type Boolean) (WantActionOnPlayer :type Boolean) (NeedToStartDialog :type Boolean) (SearchInCertainPoints :type Boolean))
  (Blackboard|BBSetStartDialogInstantly StartDialogInstantly)
  (Blackboard|BBSetWantActiononPlayer WantActionOnPlayer)
  (Blackboard|BBSetNeedtoStartDialog NeedToStartDialog)
  (Blackboard|BBSetSearchinCertainPoints SearchInCertainPoints))

(fn BBMovingConditionSetter
  (params (GoBetweenPoints :type Boolean) (MoveBetweenPointsСonsistently :type Boolean) (InRegularMode :type Boolean) (NeedToWait :type Boolean))
  (Blackboard|BBSetGoBetweenPoints GoBetweenPoints)
  (Blackboard|BBSetMoveBetweenPointsСonsistently MoveBetweenPointsСonsistently)
  (Blackboard|BBSetinRegularMode InRegularMode)
  (Blackboard|BBSetNeedtoWait NeedToWait))

(fn BBSetStartDialogwithThisReplic
  (params (StartDialogWithThisReplic :type Name))
  (Class|BlackboardComponent|SetValueasName (AI|GetBlackboard 0) (Utilities|Name|MakeLiteralName "StartDialogWithThisReplic") StartDialogWithThisReplic))