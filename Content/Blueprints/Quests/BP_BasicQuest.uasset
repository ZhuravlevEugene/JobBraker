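; BP_BasicQuest is a quest manager that registers itself on the Player at BeginPlay and tracks inventory pickup objectives.
; For inventory-type quests, each pickup event decrements the required count, flags InventoryComplete at zero and prints a completion message.
; The matching-item check is only printed and does not gate the count.
; Reads always use the first QuestBranches entry, while write-back removes and sets at CurreentQuestNum.
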(event EventBeginPlay
  (bind _asplayer (Utilities|Casting|CastToPlayer (Game|GetPlayerCharacter 0)))
  (Variables|/Game/Blueprints/Player.Player_C|SetQuestManager _asplayer self))

(event EventAddedtoInventory
  (params (Pickable :type BP%20Base%20Pickable%20Object%20Reference))
  (switch Utilities|FlowControl|Switch|SwitchonE_ActivityType (.typeofactivity (CallFunction|GetCurrentQuestStructure))
    (:NewEnumerator2
      (bind _founded (CallFunction|AddedtoInventoryIsCorrect Pickable))
      (Development|PrintString (Utilities|String|ToString(Boolean) _founded))
      (bind _zero (CallFunction|RecalcNumOfAddedtoInventory))
      (if _zero
        (bind _complete (CallFunction|CheckFoQuestComplete))
        (if _complete
          (Development|PrintString "QuestCompleted!" true true "(R=0.000000,G=0.000000,B=0.000000,A=1.000000)"))))))

(fn ConstructionScript)

(fn AddedtoInventoryIsCorrect
  (params (Item :type BP%20Base%20Pickable%20Object%20Reference))
  (bind _array_element (Utilities|Array|ForEachLoopwithBreak (.pickabletoinventory (CallFunction|GetCurrentQuestStructure)))
    (:LoopBody
      (if (== Item _array_element)
        (return true)))
    (:Completed
      (return false))))

(fn GetCurrentQuestStructure
  (return (Utilities|Array|Get(acopy) (Variables|Default|GetQuestBranches))))

(fn RecalcNumOfAddedtoInventory
  (bind _curquest (CallFunction|GetCurrentQuestStructure))
  (bind _curquest_2 (CallFunction|GetCurrentQuestStructure))
  (bind _curquest_3 (CallFunction|GetCurrentQuestStructure))
  (bind _structout (Utilities|Struct|SetmembersinS_QuestStructure (Utilities|Struct|MakeS_QuestStructure (.id _curquest_3) (.questname _curquest_3) (.description _curquest_3) (.typeofactivity _curquest_3) (.restrict _curquest_3) (.completed _curquest_3) (.inprogress _curquest_3) (.actorstointeract _curquest_3) (.classestointeract _curquest_3) (.pickabletoinventory _curquest_3) (- (.numofaddedtoinventory _curquest_3) 1) false (.pickabletograb _curquest_3) (.pickabletodrop _curquest_3) (.eventtags _curquest_3) (.nextquestname _curquest_3))))
  (CallFunction|ReplaceStructinArray _structout)
  (if (== (.numofaddedtoinventory (CallFunction|GetCurrentQuestStructure)) 0)
    (bind _structout_2 (Utilities|Struct|SetmembersinS_QuestStructure (Utilities|Struct|MakeS_QuestStructure (.id _curquest) (.questname _curquest) (.description _curquest) (.typeofactivity _curquest) (.restrict _curquest) (.completed _curquest) (.inprogress _curquest) (.actorstointeract _curquest) (.classestointeract _curquest) (.pickabletoinventory _curquest) (.numofaddedtoinventory _curquest) true (.pickabletograb _curquest) (.pickabletodrop _curquest) (.eventtags _curquest) (.nextquestname _curquest))))
    (CallFunction|ReplaceStructinArray _structout_2)
    (Development|PrintString (Utilities|String|Append (Utilities|String|ToString(Integer) (.numofaddedtoinventory _curquest_2)) (Utilities|String|ToString(Boolean) (.inventorycomplete _curquest_2))) true true "(R=1.000000,G=0.151505,B=0.000000,A=1.000000)")
    (return true)
    (else
      (return false))))

(fn CheckFoQuestComplete
  (if (.inventorycomplete (CallFunction|GetCurrentQuestStructure))
    (return true)
    (else
      (return false))))

(fn ReplaceStructinArray
  (params (Item :type S%20Quest%20Structure%20Structure%20%28by%20ref%29))
  (bind _questbranches (Variables|Default|GetQuestBranches))
  (Utilities|Array|RemoveItem _questbranches (Utilities|Array|Get(acopy) _questbranches (Variables|Default|GetCurreentQuestNum)))
  (Utilities|Array|SetArrayElem (Variables|Default|GetQuestBranches) (Variables|Default|GetCurreentQuestNum) Item))