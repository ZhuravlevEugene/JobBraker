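; Interactable safe prop whose door toggles open and closed on Interaction, unless it is locked.
; A locked safe blinks its ColorButton red three times; an unlocked one turns it green and opens after a short delay, or resets it when closing.
; The DoorRotator timeline lerps the door toward EndRotation, with interaction blocked until it finishes.
; The construction script poses the door from SafeIsOpen.
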(event Custom|OpenSafeDoor
  (if (Variables|Default|GetSafeLocked)
    (Rendering|Material|SetMaterial (Variables|Default|GetColorButton) 0 "/Game/Blueprints/Calsses/Props/BaseProp/SafeBox/M_Red.M_Red")
    (Utilities|FlowControl|Delay 0.4)
    (Rendering|Material|SetMaterial (Variables|Default|GetColorButton) 0 "/Game/StarterContent/Materials/M_Basic_Floor.M_Basic_Floor")
    (Utilities|FlowControl|Delay 0.1)
    (Rendering|Material|SetMaterial (Variables|Default|GetColorButton) 0 "/Game/Blueprints/Calsses/Props/BaseProp/SafeBox/M_Red.M_Red")
    (Utilities|FlowControl|Delay 0.4)
    (Rendering|Material|SetMaterial (Variables|Default|GetColorButton) 0 "/Game/StarterContent/Materials/M_Basic_Floor.M_Basic_Floor")
    (Utilities|FlowControl|Delay 0.1)
    (Rendering|Material|SetMaterial (Variables|Default|GetColorButton) 0 "/Game/Blueprints/Calsses/Props/BaseProp/SafeBox/M_Red.M_Red")
    (Utilities|FlowControl|Delay 0.4)
    (Rendering|Material|SetMaterial (Variables|Default|GetColorButton) 0 "/Game/StarterContent/Materials/M_Basic_Floor.M_Basic_Floor")
    (elif (Variables|Default|GetSafeIsOpen)
      (Variables|Default|SetEndRotation "0,90.000000, 0")
      (Variables|Default|SetSafeIsOpen false)
      (Variables|Default|SetCanBeInteractedWith false)
      (bind _driver (Timeline|DoorRotator PlayFromStart)
        (:Update
          (Transformation|SetRelativeRotation (Variables|Default|GetDoor) (Math|Rotator|Lerp(Rotator) (Variables|/Script/Engine.SceneComponent|GetRelativeRotation (Variables|Default|GetDoor)) (Variables|Default|GetEndRotation) _driver) false false)
          (Rendering|Material|SetMaterial (Variables|Default|GetColorButton) 0 "/Game/StarterContent/Materials/M_Basic_Floor.M_Basic_Floor"))
        (:Finished
          (Variables|Default|SetCanBeInteractedWith true)))
      (else
        (Variables|Default|SetEndRotation "0,-40.000000, 0")
        (Rendering|Material|SetMaterial (Variables|Default|GetColorButton) 0 "/Game/Blueprints/Calsses/Props/BaseProp/SafeBox/M_Green.M_Green")
        (Variables|Default|SetSafeIsOpen true)
        (Variables|Default|SetCanBeInteractedWith false)
        (Utilities|FlowControl|Delay 0.6)
        (Timeline|DoorRotator PlayFromStart)))))

(event EventInteraction
  (if (Variables|Default|GetCanBeInteractedWith)
    (CallFunction|OpenSafeDoor)))

(fn ConstructionScript
  (bind _door (Variables|Default|GetDoor))
  (|CallParentFunction)
  (if (Variables|Default|GetSafeIsOpen)
    (bind _output_get (Variables|Default|SetEndRotation "0,-40.000000, 0"))
    (Transformation|SetRelativeRotation _door _output_get false false)
    (else
      (bind _output_get_2 (Variables|Default|SetEndRotation "0,90.000000, 0"))
      (Transformation|SetRelativeRotation _door _output_get_2 false false))))