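; Boss NPC that patrols between target points, periodically heads to the GlassRoom, and confronts the player on sight.
; A tick-driven timer pauses patrol for the room trip while re-enabling player search immediately, then resumes patrol whether the move succeeds or fails.
; Pawn sensing interrupts this, sends the boss to the player and starts a dialog.
; Hardcoded dialog selection checks LevelControl's glasses events first, then the player's location.
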(event OnSeePawn(PawnSensing)
  (params (Pawn :type Pawn%20Object%20Reference))
  ;[1 1 1] Если увидел игрока
  (bind _asplayer (Utilities|Casting|CastToPlayer Pawn))
  (CallFunction|DropCheckTimer false)
  (Variables|Default|SetContinueMoveBetweenTargets false)
  (Variables|Default|SetSearchingForPlayer false)
  (Variables|Default|SetMovingToPlayer true)
  (Variables|Default|SetMoveBetweenTargetPoints false)
  (CallFunction|SetPawnSensing false)
  (Class|NavMovementComponent|StopActiveMovement (Variables|Character|GetCharacterMovement))
  (AI|AIMoveTo self "0, 0, 0" _asplayer 15.0 false
    (:OnSuccess
      (CallFunction|StartDialog (CallFunction|ChooseDialog) true))))

(event EventBeginPlay
  (|CallParentFunction) ; This node is disabled and will not be called.\nDrag off pins to build functionality.
)

(event EventTick
  (params (DeltaSeconds :type Float%20%28single-precision%29))
  (|CallParentFunction DeltaSeconds)
  (if (Variables|Default|GetUseCheckTimer)
    (bind _timerend (CallFunction|CalculateCheckTimer))
    (if _timerend
      (Variables|Default|SetCheckTimer 0.0)
      (Variables|Default|SetMoveBetweenTargetPoints false)
      (Variables|Default|SetContinueMoveBetweenTargets false)
      (bind _movementresult (AI|AIMoveTo self "0, 0, 0" (Variables|Default|GetGlassRoom) 5.0 false)
        (:then
          ;[1 1 1] Включаем поиск игрока, потому что нужно в первую очередь найти его, а не дойти до нужной комнаты
          (CallFunction|StartSearchforPlayer true true))
        (:OnSuccess
          (Utilities|FlowControl|Delay 2.0)
          (Variables|Default|SetUseCheckTimer true)
          (Variables|Default|SetContinueMoveBetweenTargets true)
          (Variables|Default|SetMoveBetweenTargetPoints true)
          (CallFunction|StartSearchforPlayer true true))
        (:OnFail
          ;[1 1 1] Если цель недостижима, то посылаем посылаем искать игрока
          (Development|PrintString (Utilities|String|Append "I stop movement because of:    " (Utilities|String|EnumtoString _movementresult)) true true "(R=1.000000,G=0.000000,B=0.066903,A=1.000000)" 1e+01)
          (Variables|Default|SetUseCheckTimer true)
          (Variables|Default|SetContinueMoveBetweenTargets true)
          (Variables|Default|SetMoveBetweenTargetPoints true)
          (CallFunction|StartSearchforPlayer true true))))))

(fn ConstructionScript
  (|CallParentFunction))

(fn CalculateCheckTimer
  (bind _output_get (Variables|Default|SetCheckTimer (+ (Variables|Default|GetCheckTimer) (Utilities|Time|GetWorldDeltaSeconds))))
  (if (>= _output_get (Variables|Default|GetCheckTimerDelay))
    (Variables|Default|SetUseCheckTimer false)
    (return true)
    (else
      (return false))))

(fn ChooseDialog
  ;[1 1 1] Это захардкоженная функция. Можно применять только в нужном месте
  (bind _array_element (Utilities|Array|ForEachLoopwithBreak (Variables|/Game/Blueprints/Calsses/LevelControl/LevelControls/LevelControlBase.LevelControlBase_C|GetSpecialEvents (Variables|Default|GetLevelControl)) :!label _label)
    (:LoopBody
      (switch string _array_element
        (:GlassesPlugged
          (LocalVariables|SetL_DialogReplic "R6")
          (LocalVariables|SetL_ReplicFounded true)
          (goto _label Break))
        (:GlassesDestroyed
          (LocalVariables|SetL_DialogReplic "R1")
          (LocalVariables|SetL_ReplicFounded true)
          (goto _label Break))))
    (:Completed
      (if (LocalVariables|GetL_ReplicFounded)
        (return (LocalVariables|GetL_DialogReplic))
        (elif (Utilities|Name|Equal(Name) (Variables|/Game/Blueprints/Calsses/LevelControl/LevelControls/LevelControlBase.LevelControlBase_C|GetCurrentPlayerLocation (Variables|Default|GetLevelControl)) "GlassRoom")
          (return "WorkChecking")
          (else
            (return "WC_NotInGlassRoom")))))))

(fn DropCheckTimer
  (params (TurnOn :type Boolean))
  (Variables|Default|SetUseCheckTimer TurnOn)
  (Variables|Default|SetCheckTimer 0.0)
  (return (Variables|Default|GetUseCheckTimer)))

(fn StartSearchforPlayer
  (params (SearchingForPlayer :type Boolean) (bSeePawns :type Boolean))
  (CallFunction|SetPawnSensing bSeePawns)
  (Variables|Default|SetSearchingForPlayer SearchingForPlayer))