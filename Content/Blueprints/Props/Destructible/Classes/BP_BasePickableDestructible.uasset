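; Base pickable prop that shatters on hard impacts and delegates inventory add and remove to its parent class.
; Its static mesh breaks when hit at or above a critical speed, if destruction is allowed, including a check for the plugged state.
; Breaking releases it from the player's physics handle, then swaps it for a spawned destructible actor fractured by impulse and radial damage.
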(event OnComponentHit(Undestructible)
  (params (HitComponent :type Primitive%20Component%20Object%20Reference) (OtherActor :type Actor%20Object%20Reference) (OtherComp :type Primitive%20Component%20Object%20Reference) (NormalImpulse :type Vector :default "0, 0, 0") (Hit :type Hit%20Result%20Structure%20%28by%20ref%29))
  (bind (_bblockinghit _binitialoverlap _time _distance _location _impactpoint _normal) (Collision|BreakHitResult Hit))
  (bind _undestructible (Variables|Default|GetUndestructible))
  (if (Variables|Default|GetCanBeDestruct)
    (if (Variables|Default|GetPlugged)
      (if (Variables|Default|GetCanBeDestructWhilePlugged)
        (if (>= (Math|Vector|VectorLength (Transformation|GetComponentVelocity HitComponent)) (Variables|Default|GetCriticalDamageHit)) :!label _label
          (CallFunction|RemoveDestructiblefromPlayer _undestructible)
          (bind _returnvalue (Game|SpawnActorfromClass "/Script/ApexDestruction.DestructibleActor" (Transformation|GetWorldTransform _undestructible) "AlwaysSpawn" 0 0))
          (Class|DestructibleComponent|SetDestructibleMesh (Variables|/Script/ApexDestruction.DestructibleActor|GetDestructibleComponent _returnvalue) (Variables|Default|GetDestructibleMesh))
          (Components|DestroyComponent (Variables|Default|GetUndestructible))
          (Physics|SetSimulatePhysics (Variables|/Script/ApexDestruction.DestructibleActor|GetDestructibleComponent _returnvalue) true)
          (Physics|AddImpulse (Variables|/Script/ApexDestruction.DestructibleActor|GetDestructibleComponent _returnvalue) _normal "None" false)
          (Class|DestructibleComponent|ApplyRadiusDamage (Variables|/Script/ApexDestruction.DestructibleActor|GetDestructibleComponent _returnvalue) 1e+03 _location 2e+02 1.0 true)))
      (else
        (goto _label)))))

(event OnComponentFracture(Destructible)
  (params (HitPoint :type Vector%20%28by%20ref%29 :default "0, 0, 0") (HitDirection :type Vector%20%28by%20ref%29 :default "0, 0, 0"))
  (CallFunction|LetGofromPlayer (Variables|Default|GetDestructible)))

(event EventRemovefromInventory
  (params (Destroy :type Boolean) (NewLocation :type Vector :default "0, 0, 0") (Target :type Primitive%20Component%20Object%20Reference))
  (|CallParentFunction Destroy NewLocation (Variables|Default|GetUndestructible)))

(event EventAddtoInventory
  (params (Target :type Primitive%20Component%20Object%20Reference))
  (|CallParentFunction (Variables|Default|GetUndestructible)))

(fn ConstructionScript
  (|CallParentFunction)
  (Components|StaticMesh|SetStaticMesh (Variables|Default|GetUndestructible) (Variables|Default|GetUndestructibleMesh)))

(fn RemoveDestructiblefromPlayer
  (params (Component :type Object%20Object%20Reference))
  (bind _asplayer (Utilities|Casting|CastToPlayer (Game|GetPlayerCharacter 0)))
  (bind _output_get (Variables|Default|SetPlayer _asplayer))
  (if (== (Class|PhysicsHandleComponent|GetGrabbedComponent (Variables|/Game/Blueprints/Player.Player_C|GetPhysicsHandle _output_get)) Component)
    (Variables|/Game/Blueprints/Player.Player_C|SetIsGrabbing (Variables|Default|GetPlayer) false)
    (Physics|Components|PhysicsHandle|ReleaseComponent (Variables|/Game/Blueprints/Player.Player_C|GetPhysicsHandle (Variables|Default|GetPlayer)))
    (Variables|/Game/Blueprints/Player.Player_C|SetGrabbedComponent (Variables|Default|GetPlayer) 0)))