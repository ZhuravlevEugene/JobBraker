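; A basic game mode that tracks a level's task list and marks tasks as completed.
; LevelControlInteraction prints the incoming task, finds the identical struct in LevelTasks and writes it back with Done set to true, keeping its other fields.
; A disconnected debug loop would print all tasks in reverse, colored by completion.
; Tick and ChangeTaskStatus are empty.
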(event EventLevelControlInteraction
  (params (CompletedTask :type S%20Level%20Tasks%20Structure))
  (bind (_task _done _actortag _taskactivity) (Utilities|Struct|BreakS_LevelTasks CompletedTask))
  (bind _leveltasks (Variables|Default|GetLevelTasks))
  (bind _leveltasks_2 (Variables|Default|GetLevelTasks))
  (bind _returnvalue (Utilities|Array|FindItem _leveltasks CompletedTask))
  (bind _output (Utilities|Array|Get(acopy) _leveltasks_2 _returnvalue))
  (bind (_task_2 _done_2 _actortag_2 _taskactivity_2) (Utilities|Struct|BreakS_LevelTasks _output))
  (Development|PrintString (Utilities|String|Append (Utilities|String|ToString(Text) _task) (Utilities|String|ToString(Boolean) _done) (Utilities|String|ToString(Name) _actortag) (Utilities|String|ToString(Text) _taskactivity)) true true "(R=0.000000,G=0.660000,B=1.000000,A=1.000000)" 1e+03)
  (bind _structout (Utilities|Struct|SetmembersinS_LevelTasks (Utilities|Struct|MakeS_LevelTasks _task_2 true _actortag_2 _taskactivity_2)))
  (Utilities|Array|SetArrayElem _leveltasks_2 _returnvalue _structout))

(event EventTick
  (params (DeltaSeconds :type Float%20%28single-precision%29)))

(fn ConstructionScript)

(fn ChangeTaskStatus)