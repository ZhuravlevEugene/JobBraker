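; Timer component that counts elapsed time and notifies its owning actor when a delay runs out.
; While UseTimer is on, Tick adds world delta seconds to Timer and compares it to TimerDelay.
; At the delay, only if StopTimerAtOff is set, RetriggerTimer zeroes and disables the timer, then TimerOff calls TimerStopedMessage on the owner.
; Despite its name, RetriggerTimer does not restart counting.
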(event Custom|TimerOff
  (Class|ITimer|TimerStoped(Message) (Components|GetOwner)))

(event EventTick
  (params (DeltaSeconds :type Float%20%28single-precision%29))
  (if (Variables|Default|GetUseTimer)
    (bind _output_get (Variables|Default|SetTimer (+ (Variables|Default|GetTimer) (Utilities|Time|GetWorldDeltaSeconds))))
    (if (>= _output_get (Variables|Default|GetTimerDelay))
      (if (Variables|Default|GetStopTimerAtOff)
        (CallFunction|RetriggerTimer)
        (CallFunction|TimerOff)))))

(fn RetriggerTimer
  (Variables|Default|SetTimer 0.0)
  (Variables|Default|SetUseTimer false))