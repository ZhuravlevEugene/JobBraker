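; Boss NPC that periodically checks on the player's work and confronts them with dialogue, building on a parent NPC class.
; A Tick timer sends it to the GlassRoom-tagged target point in search mode, and MoveToCabinet returns it to BossCabinet and re-arms the timer.
; When the parent's stop-while-searching event fires, it approaches the player and picks dialogue from LevelControl's special events, defaulting to a work-check line when none exist.
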(event Custom|MoveToCabinet
  (bind _array_element (Utilities|Array|ForEachLoopwithBreak (Variables|Default|GetTargetPointsArray))
    (:LoopBody
      (if (Actor|ActorHasTag _array_element "BossCabinet")
        (AI|AIMoveTo self "0, 0, 0" _array_element 1e+01 false
          (:then
            (Variables|Default|SetUseCheckTimer true)
            (Variables|Default|SetCheckTimerDelay 1e+01)
            (Variables|Default|SetMovingToPlayer false)
            (Variables|Default|SetSearchingForPlayer false)))))))

(event EventBeginPlay
  (|CallParentFunction) ; This node is disabled and will not be called.\nDrag off pins to build functionality.
)

(event Collision|EventActorBeginOverlap
  (params (OtherActor :type Actor%20Object%20Reference)))

(event EventTick
  (params (DeltaSeconds :type Float%20%28single-precision%29))
  (|CallParentFunction DeltaSeconds)
  (if (Variables|Default|GetUseCheckTimer)
    (bind _output_get (Variables|Default|SetCheckTimer (+ (Variables|Default|GetCheckTimer) DeltaSeconds)))
    (if (>= _output_get (Variables|Default|GetCheckTimerDelay))
      (Variables|Default|SetCheckTimer 0.0)
      (Variables|Default|SetUseCheckTimer false)
      (bind _array_element (Utilities|Array|ForEachLoopwithBreak (Variables|Default|GetTargetPointsArray))
        (:LoopBody
          (if (Actor|ActorHasTag _array_element "GlassRoom")
            (Variables|Default|SetSearchingForPlayer true)
            (Variables|Default|SetPlayerSearchingReason "CheckWork")
            (Class|NavMovementComponent|StopActiveMovement (Variables|Character|GetCharacterMovement))
            (bind _movementresult (AI|AIMoveTo self "0, 0, 0" _array_element 1e+01 false)
              (:OnFail
                (switch Utilities|FlowControl|Switch|SwitchonEPathFollowingResult _movementresult
                  (:Success
                    _)
                  (:Blocked
                    _)
                  (:OffPath
                    _)
                  (:Aborted
                    _)
                  (:Invalid
                    _))
                (Development|PrintString (Utilities|String|Append "I STOP MOVEMENT TO:   " (Utilities|GetDisplayName _array_element) " 
Reason:   " (Utilities|String|EnumtoString _movementresult)))))))))))

(event EventStopMoveifSearchingPlayer
  (bind _levelcontrol (Variables|Default|GetLevelControl))
  (bind _specialevents (Variables|/Game/Blueprints/Calsses/LevelControl/LevelControls/LevelControlBase.LevelControlBase_C|GetSpecialEvents _levelcontrol))
  (|CallParentFunction)
  (if (not (Variables|Default|GetMovingToPlayer))
    (switch string (Variables|Default|GetPlayerSearchingReason)
      (:CheckWork
        (if (> (Utilities|Array|Length _specialevents) 0)
          (bind _array_element (Utilities|Array|ForEachLoopwithBreak _specialevents :!label _label)
            (:LoopBody
              (switch string _array_element
                (:GlassDestroyed
                  (Variables|Default|SetMovingToPlayer true)
                  (CallFunction|MoveandStartDialog "R1")
                  (goto _label Break))
                (:PlugPortUsed
                  (Variables|Default|SetMovingToPlayer true)
                  (CallFunction|MoveandStartDialog "R6")
                  (goto _label Break)))))
          (else
            (Variables|Default|SetMovingToPlayer true)
            (bind _movementresult (AI|AIMoveTo self "0, 0, 0" (Variables|Default|GetPlayer) 5.0 false)
              (:OnSuccess
                (CallFunction|ChooseDialog)
                (CallFunction|StartDialog "None" true))
              (:OnFail
                (Development|PrintString (Utilities|String|Append "NPC: Cant find the way! Because of:     " (Utilities|String|EnumtoString _movementresult)) true true "(R=1.000000,G=0.000000,B=0.087363,A=1.000000)" 1e+01)))))))))

(fn ConstructionScript
  (|CallParentFunction))

(fn ChooseDialog
  (bind _levelcontrol (Variables|Default|GetLevelControl))
  (bind _specialevents (Variables|/Game/Blueprints/Calsses/LevelControl/LevelControls/LevelControlBase.LevelControlBase_C|GetSpecialEvents _levelcontrol))
  (if (> (Utilities|Array|Length _specialevents) 0)
    (bind _array_element (Utilities|Array|ForEachLoopwithBreak _specialevents :!label _label)
      (:LoopBody
        (switch string _array_element
          (:GlassDestroyed
            (Variables|Default|SetMovingToPlayer true)
            (Variables|Default|SetStartedReplic "R1")
            (goto _label Break))
          (:GlassesPlugged
            (Variables|Default|SetMovingToPlayer true)
            (Variables|Default|SetStartedReplic "R6")
            (goto _label Break)))))
    (else
      (Variables|Default|SetMovingToPlayer true)
      (Variables|Default|SetStartedReplic "WorkChecking"))))