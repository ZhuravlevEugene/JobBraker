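; Base NPC character that runs a starting activity (random or sequential patrol, waiting, or no behavior tree) and can open dialogs with the player.
; BeginPlay passes the reaction flag and activity to BaseNPCController, which exposes behavior-tree branches and blackboard.
; MoveAndStartDialog only walks to a free player; StartDialog opens the window and halts the player.
; Older sensing and dialog-queue logic is disconnected; Tick prints a debug flag.
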(event OnSeePawn(PawnSensing)
  (params (Pawn :type Pawn%20Object%20Reference)))

(event Custom|MoveAndStartDialog
  (params (StartedReplic :type Name))
  (Variables|DialogSystem|SetStartedReplic StartedReplic)
  (if (Variables|/Game/Blueprints/Player.Player_C|GetInDialog (Variables|Default|GetPlayer))
    ;[1 1 1] Старая логика на случай дублирования диалога
    (Variables|Default|SetCheckForPlayerDialogUpdate true)
    (else
      (bind _movementresult (AI|AIMoveTo self "0, 0, 0" (Variables|Default|GetPlayer) 35.0 false)
        (:OnFail
          (Development|PrintString (Utilities|String|Append "NPC: Cant find the way! Because of:     " (Utilities|String|EnumtoString _movementresult)) true true "(R=1.000000,G=0.000000,B=0.087363,A=1.000000)" 1e+01))))))

(event Custom|StopMoveIfSearchingPlayer
  ;[1 1 1] Старая логика, но может пригодиться (перенести в функцию)
)

(event EventTick
  (params (DeltaSeconds :type Float%20%28single-precision%29))
  (Development|PrintString (Utilities|String|Append "CanReactToPlayer:    " (Utilities|String|ToString(Boolean) (ScalableFloat|GetValueasBool (AI|GetBlackboard (CallFunction|GetCastedController)) (Utilities|Name|MakeLiteralName "CanReactToPlayer")))) true true "(R=0.000000,G=0.660000,B=1.000000,A=1.000000)" 0.0))

(event EventBeginPlay
  ;[1 1 1] Запись левел контрол в переменную
  (Default|BBSetCanReacttoPlayer (CallFunction|GetCastedController) (Variables|CunstructionParametrs|GetNPCCanReactToPlayer))
  (Variables|Default|SetPlayer (.AsPlayer (Utilities|Casting|CastToPlayer (Game|GetPlayerCharacter 0))))
  (bind _outactors (Actor|GetAllActorsOfClass "/Game/Blueprints/Calsses/LevelControl/LevelControls/LevelControlBase.LevelControlBase_C"))
  (bind _array_element (Utilities|Array|ForEachLoopwithBreak _outactors :!label _label)
    (:LoopBody
      (Variables|Default|SetLevelControl _array_element)
      (goto _label Break))
    (:Completed
      (switch Utilities|FlowControl|Switch|SwitchonE_ActivityType (Variables|CunstructionParametrs|GetStartedActivity)
        (:NewEnumerator7
          (Default|GoBetweenPointsBranch (CallFunction|GetCastedController) 2.0 true 0.0))
        (:NewEnumerator8
          (Default|GoBetweenPointsBranch (CallFunction|GetCastedController) 2.0 false 0.0))
        (:NewEnumerator9
          (Default|MoveandWaitBranch (CallFunction|GetCastedController) (Variables|Waiting|GetWaitingPoint) (Variables|Waiting|GetRotatePoint) 0.0))
        (:NewEnumerator11
          (Default|BreakBehaviorTree (CallFunction|GetCastedController) 0.0))))))

(fn ConstructionScript
  (Rendering|Components|TextRender|SetText (Variables|Default|GetTextRender) (Variables|CunstructionParametrs|GetRoleText))
  (Default|BBSetCanReacttoPlayer (CallFunction|GetCastedController) (Variables|CunstructionParametrs|GetNPCCanReactToPlayer)))

(fn StartDialog
  (params (Dialog :type Name) (RotatePlayerToNPC :type Boolean))
  (bind _player (Variables|Default|GetPlayer))
  (if (Utilities|Name|NotEqual(Name) Dialog "None")
    (Variables|DialogSystem|SetStartedReplic Dialog))
  (Default|OpenDialogVindow (Variables|Default|GetPlayer) (Variables|DialogSystem|GetStartedReplic) (Variables|CunstructionParametrs|GetNPCRole) self)
  (Variables|/Game/Blueprints/Player.Player_C|SetLocationOfTarget _player (+ (Transformation|GetWorldLocation (Variables|Character|GetMesh)) "0, 0,85.000000")) ; Для поворота ГГ на НПС
  (Variables|/Game/Blueprints/Player.Player_C|SetCalculatingTimer _player RotatePlayerToNPC)
  (Default|SetMaxWalkSpeed _player 0.0)
  (Variables|/Game/Blueprints/Player.Player_C|SetInDialog _player true)
  (Variables|DialogSystem|SetInDialog true :!pinned true) ; УБРАТЬ В БУДУЩЕМ \n(так как есть блекборд)
  (Variables|/Game/Blueprints/Player.Player_C|SetInDialogWith _player 0))

(fn ChooseRandomTargetPont
  (params (TargetPointArray :type Array%20of%20Target%20Point%20Object%20References))
  (bind _output_get (LocalVariables|SetL_TargetPoints TargetPointArray))
  (return (Utilities|Array|Get(acopy) _output_get (Math|Random|RandomIntegerinRange 0 (- (Utilities|Array|Length (LocalVariables|GetL_TargetPoints)) 1)))))

(fn GetCastedController
  (return (.AsBase%20NPCController (Utilities|Casting|CastToBaseNPCController (Pawn|GetController)))))