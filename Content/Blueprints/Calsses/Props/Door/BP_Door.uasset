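; Lockable hinged door that toggles on interaction and opens automatically when a BaseNPC overlaps its trigger.
; A timeline lerps the 90-degree swing with door collision disabled, restoring it on finish.
; NavCollision is moved and sized to the open leaf, or collapsed to zero when closed; the construction script applies the same setup for the initial state.
; Toggling sends optional named open or close events to LevelControl.
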(event OnComponentBeginOverlap(OpenCollision)
  (params (OverlappedComponent :type Primitive%20Component%20Object%20Reference) (OtherActor :type Actor%20Object%20Reference) (OtherComp :type Primitive%20Component%20Object%20Reference) (OtherBodyIndex :type Integer) (bFromSweep :type Boolean) (SweepResult :type Hit%20Result%20Structure%20%28by%20ref%29))
  (Utilities|Casting|CastToBaseNPC OtherActor)
  (if (not (Variables|DoorSetup|GetDoorLocked))
    (if (not (Variables|DoorSetup|GetDoorIsOpen))
      (CallFunction|OpenDoor))))

(event Custom|OpenDoor
  (if (not (Variables|DoorSetup|GetDoorLocked))
    (if (Variables|DoorSetup|GetDoorIsOpen)
      (Variables|DoorSetup|SetDoorIsOpen false)
      (Variables|DoorSetup|SetStartDoor "0,-90.000000, 0")
      (Variables|DoorSetup|SetEndDoor "0, 0, 0")
      (CallFunction|SendEventifNeed (Variables|Default|GetCloseEvent))
      (else
        (Variables|DoorSetup|SetDoorIsOpen true)
        (Variables|DoorSetup|SetStartDoor "0, 0, 0")
        (Variables|DoorSetup|SetEndDoor "0,-90.000000, 0")
        (CallFunction|SendEventifNeed (Variables|Default|GetOpenEvent))))
    (Collision|SetCollisionEnabled (Variables|Default|GetDoor) "NoCollision")
    (bind _driver (Timeline|DoorRotator PlayFromStart)
      (:Update
        (Transformation|SetRelativeRotation (Variables|Default|GetDoor) (Math|Rotator|Lerp(Rotator) (Variables|DoorSetup|GetStartDoor) (Variables|DoorSetup|GetEndDoor) _driver) false false))
      (:Finished
        (if (Variables|DoorSetup|GetDoorIsOpen)
          (Transformation|SetRelativeTransform (Variables|Default|GetNavCollision) (Math|Transform|MakeTransform "-50.000000,50.000000,95.000000" (Variables|/Script/Engine.SceneComponent|GetRelativeRotation (Variables|Default|GetNavCollision))) false false)
          (Components|Box|SetBoxExtent (Variables|Default|GetNavCollision) "50.000000,2.000000,90.000000" true)
          (Collision|SetCollisionEnabled (Variables|Default|GetDoor) "QueryAndPhysics")
          (else
            (Transformation|SetRelativeTransform (Variables|Default|GetNavCollision) (Math|Transform|MakeTransform "0.000000,50.000000,95.000000" (Variables|/Script/Engine.SceneComponent|GetRelativeRotation (Variables|Default|GetNavCollision))) false false)
            (Components|Box|SetBoxExtent (Variables|Default|GetNavCollision) "0, 0, 0" true)
            (Collision|SetCollisionEnabled (Variables|Default|GetDoor) "QueryAndPhysics")))))))

(event EventBeginPlay
  (bind _levelcontrol (CallFunction|GetLevelControl))
  (Variables|Default|SetLevelControl _levelcontrol))

(event EventInteraction
  (CallFunction|OpenDoor))

(fn ConstructionScript
  (if (Variables|DoorSetup|GetDoorIsOpen)
    (Transformation|SetRelativeRotation (Variables|Default|GetDoor) "0,-90.000000, 0" false false)
    (Variables|DoorSetup|SetStartDoor "0,-90.000000, 0")
    (Variables|DoorSetup|SetEndDoor "0, 0, 0")
    (Transformation|SetRelativeTransform (Variables|Default|GetNavCollision) (Math|Transform|MakeTransform "-50.000000,50.000000,95.000000" (Variables|/Script/Engine.SceneComponent|GetRelativeRotation (Variables|Default|GetNavCollision))) false false)
    (Components|Box|SetBoxExtent (Variables|Default|GetNavCollision) "50.000000,2.000000,90.000000" true)
    (else
      (Transformation|SetRelativeRotation (Variables|Default|GetDoor) "0, 0, 0" false false)
      (Variables|DoorSetup|SetStartDoor "0, 0, 0")
      (Variables|DoorSetup|SetEndDoor "0,-90.000000, 0")
      (Transformation|SetRelativeTransform (Variables|Default|GetNavCollision) (Math|Transform|MakeTransform "0.000000,50.000000,95.000000" (Variables|/Script/Engine.SceneComponent|GetRelativeRotation (Variables|Default|GetNavCollision))) false false)
      (Components|Box|SetBoxExtent (Variables|Default|GetNavCollision) "0, 0, 0" true))))

(fn SendEventifNeed
  (params (Event :type String))
  (if (> (Utilities|String|Len Event) 0)
    (Default|LevelEvent (Variables|Default|GetLevelControl) Event (Utilities|Array|MakeArray ""))))