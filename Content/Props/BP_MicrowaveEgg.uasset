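; BP_MicrowaveEgg is an interactable prop that sets off a one-time particle burst after being interacted with enough times.
; Each Interaction event increments a click counter and compares it to a target count.
; Once the target is reached, a DoOnce activates the particle system, scales it up sharply after a delay, then switches it off and destroys StaticMesh1.
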(event EventInteraction
  (bind _output_get (Variables|Default|SetCurrentClickCount (+ (Variables|Default|GetCurrentClickCount) 1)))
  (if (>= _output_get (Variables|Default|GetTargetClickCount))
    (Utilities|FlowControl|DoOnce false
      (:Completed
        (Components|Activation|SetActive (Variables|Default|GetParticleSystem) true false)
        (Utilities|FlowControl|Delay 0.9)
        (Transformation|SetWorldScale3D (Variables|Default|GetParticleSystem) "10.000000,10.000000,10.000000")
        (Utilities|FlowControl|Delay 0.2)
        (Components|Activation|SetActive (Variables|Default|GetParticleSystem) false false)
        (Components|DestroyComponent (Variables|Default|GetStaticMesh1))))))

(fn ConstructionScript)