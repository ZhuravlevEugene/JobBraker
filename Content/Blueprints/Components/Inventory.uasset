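; Inventory component that stores Pickable items in an Items array and tracks the selected one through a CurrentItem index.
; Adding to an empty inventory selects index 0, while removing an item shifts the selection through the Up or Down events.
; UpCurrentItem and DownCurrentItem wrap at the array ends and otherwise scan forward from the neighboring index for a valid entry.
; An on-screen debug listing of the contents is present but disconnected.
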(event Custom|Add%20to%20Inventory
  (params (Pickable :type BP%20Base%20Pickable%20Object%20Reference%20%28by%20ref%29))
  (if (> (Utilities|Array|Length (Variables|Default|GetItems)) 0)
    _
    (else
      (Variables|Default|SetCurrentItem 0)))
  (Utilities|Array|Add (Variables|Default|GetItems) Pickable))

(event Custom|DownCurrentItem
  (if (== (Utilities|Array|Length (Variables|Default|GetItems)) 1)
    (Variables|Default|SetCurrentItem 0)
    (elif (== (Variables|Default|GetCurrentItem) 0)
      (Variables|Default|SetCurrentItem (- (Utilities|Array|Length (Variables|Default|GetItems)) 1))
      (else
        (bind _index (Utilities|FlowControl|ForLoopwithBreak (- (Variables|Default|GetCurrentItem) 1) (- (Utilities|Array|Length (Variables|Default|GetItems)) 1) :!label _label)
          (:LoopBody
            (Utilities|IsValid (Utilities|Array|Get(acopy) (Variables|Default|GetItems) _index)
              (:Is%20Valid
                (Variables|Default|SetCurrentItem _index)
                (goto _label Break)))))))))

(event Custom|UpCurrentItem
  (bind _items (Variables|Default|GetItems))
  (bind _returnvalue (Utilities|Array|Length _items))
  (if (== _returnvalue 1)
    (Variables|Default|SetCurrentItem 0)
    (elif (== (Variables|Default|GetCurrentItem) (- (Utilities|Array|Length (Variables|Default|GetItems)) 1))
      (Variables|Default|SetCurrentItem 0)
      (else
        (bind _index (Utilities|FlowControl|ForLoopwithBreak (+ (Variables|Default|GetCurrentItem) 1) (- _returnvalue 1) :!label _label)
          (:LoopBody
            (Utilities|IsValid (Utilities|Array|Get(acopy) (Variables|Default|GetItems) _index)
              (:Is%20Valid
                (Variables|Default|SetCurrentItem _index)
                (goto _label Break)))))))))

(event Custom|RemoveFromInventory
  (params (Pickable :type BP%20Base%20Pickable%20Object%20Reference%20%28by%20ref%29))
  (bind _items (Variables|Default|GetItems))
  (Utilities|Array|RemoveItem _items Pickable)
  (if (== (Variables|Default|GetCurrentItem) (Utilities|Array|LastIndex _items))
    (CallFunction|UpCurrentItem)
    (else
      (CallFunction|DownCurrentItem))))

(event EventTick
  (params (DeltaSeconds :type Float%20%28single-precision%29)))