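; BP_BasePickable is a base Blueprint for pickable props, handling release from the player's grab and moves in and out of inventory.
; LetGoFromPlayer resets the component's relative transform and, if the player's PhysicsHandle holds it, releases it and clears the grab state.
; Inventory storage hides nothing: it teleports the target to world origin with physics off.
; Removal either destroys the actor or teleports the target to a given location with physics back on.
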(event Custom|LetGoFromPlayer
  (params (Component :type Primitive%20Component%20Object%20Reference))
  (bind _returnvalue (Math|Transform|MakeTransform "0, 0, 0"))
  (bind _asplayer (Utilities|Casting|CastToPlayer (Game|GetPlayerCharacter 0)))
  (bind _output_get (Variables|Default|SetPlayer _asplayer))
  (if (== (Class|PhysicsHandleComponent|GetGrabbedComponent (Variables|/Game/Blueprints/Player.Player_C|GetPhysicsHandle _output_get)) Component)
    (Transformation|SetRelativeTransform Component _returnvalue false false)
    (Variables|/Game/Blueprints/Player.Player_C|SetIsGrabbing (Variables|Default|GetPlayer) false)
    (Physics|Components|PhysicsHandle|ReleaseComponent (Variables|/Game/Blueprints/Player.Player_C|GetPhysicsHandle (Variables|Default|GetPlayer)))
    (Variables|/Game/Blueprints/Player.Player_C|SetGrabbedComponent (Variables|Default|GetPlayer) 0)
    (else
      (Transformation|SetRelativeTransform Component _returnvalue false false))))

(event Custom|Add%20to%20Inventory
  (params (Target :type Primitive%20Component%20Object%20Reference))
  ;[1 1 1] Для работы с инвентарем
  (Transformation|SetWorldLocation Target "0, 0, 0" false true)
  (Physics|SetSimulatePhysics Target false))

(event Custom|RemoveFromInventory
  (params (Destroy :type Boolean) (NewLocation :type Vector) (Target :type Primitive%20Component%20Object%20Reference))
  ;[1 1 1] Для работы с инвентарем
  (if Destroy
    (Actor|DestroyActor)
    (else
      (Transformation|SetWorldLocation Target NewLocation false true)
      (Physics|SetSimulatePhysics Target true))))

(fn ConstructionScript)