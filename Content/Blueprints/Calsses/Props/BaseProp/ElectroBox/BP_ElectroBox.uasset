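; BP_ElectroBox is an electrical box prop with a switch that the Interaction event toggles on and off.
; Each toggle flips TurnedOn, picks a raised or lowered end position, and replays the Mover timeline to lerp the Switch component there from its current relative location.
; When the timeline finishes, it sends an ElectroBoxTurnedOn or ElectroBoxTurnedOff level event through LevelControl.
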(event Custom|ToggleSwitch
  (if (Variables|Default|GetTurnedOn)
    (Variables|Default|SetTurnedOn false)
    (Variables|Default|SetEndLocation "10.000000,0.000000,17.000000")
    (bind _driver (Timeline|Mover PlayFromStart)
      (:Update
        (Transformation|SetRelativeLocation (Variables|Default|GetSwitch) (Math|Vector|Lerp(Vector) (Variables|/Script/Engine.SceneComponent|GetRelativeLocation (Variables|Default|GetSwitch)) (Variables|Default|GetEndLocation) _driver) false false))
      (:Finished
        (if (Variables|Default|GetTurnedOn)
          (Default|LevelEvent (Variables|Default|GetLevelControl) "ElectroBoxTurnedOn" (Utilities|Array|MakeArray ""))
          (else
            (Default|LevelEvent (Variables|Default|GetLevelControl) "ElectroBoxTurnedOff" (Utilities|Array|MakeArray ""))))))
    (else
      (Variables|Default|SetTurnedOn true)
      (Variables|Default|SetEndLocation "10.000000,0.000000,57.000000")
      (Timeline|Mover PlayFromStart))))

(event EventInteraction
  (CallFunction|ToggleSwitch))

(fn ConstructionScript
  (|CallParentFunction))