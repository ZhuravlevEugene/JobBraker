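; Plug port prop that snaps in pickable plug actors on overlap and completes the matching level task.
; If the port is not a spent single-use one, it checks I_PlugIn and accepted tags, releases the plug from the player and disables pickup.
; Action attaches the overlapped component to AttachPoint, reports the tag-matched unfinished task to the game mode and marks it done.
; Overlap logic sits in a shared event so child classes can feed it from several colliders.
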(event OnComponentBeginOverlap(Collision)
  (params (OverlappedComponent :type Primitive%20Component%20Object%20Reference) (OtherActor :type Actor%20Object%20Reference) (OtherComp :type Primitive%20Component%20Object%20Reference) (OtherBodyIndex :type Integer) (bFromSweep :type Boolean) (SweepResult :type Hit%20Result%20Structure%20%28by%20ref%29))
  (CallFunction|Overlaped OtherActor OtherComp))

(event Custom|Action
  (params (Actor :type Actor%20Object%20Reference) (Component :type Primitive%20Component%20Object%20Reference))
  ;[1 1 1 1 12] Действие, которое выполняет класс
  (CallFunction|Attach Actor Component)
  (Variables|Default|SetIsUsing true)
  (CallFunction|SendReporttoGameMode (Variables|/Script/Engine.Actor|GetTags Actor)))

(event Custom|SendReportToGameMode
  (params (Tags :type Array%20of%20Names))
  (bind (_founded _task) (CallFunction|GetTaskbyTag Tags))
  (if _founded
    (Class|IInteract|LevelControlInteraction(Message) (Game|GetGameMode) (Utilities|Array|Get(acopy) (Variables|Default|GetTasks) (Utilities|Array|FindItem (Variables|Default|GetTasks) _task)))
    (bind _structout (Utilities|Struct|SetmembersinS_LevelTasks (Utilities|Struct|MakeS_LevelTasks (.Task (Utilities|Struct|BreakS_LevelTasks (Utilities|Array|Get(acopy) (Variables|Default|GetTasks) (Utilities|Array|FindItem (Variables|Default|GetTasks) _task)))) true (.ActorTag (Utilities|Struct|BreakS_LevelTasks (Utilities|Array|Get(acopy) (Variables|Default|GetTasks) (Utilities|Array|FindItem (Variables|Default|GetTasks) _task)))) (.TaskActivity (Utilities|Struct|BreakS_LevelTasks (Utilities|Array|Get(acopy) (Variables|Default|GetTasks) (Utilities|Array|FindItem (Variables|Default|GetTasks) _task)))))))
    (Utilities|Array|SetArrayElem (Variables|Default|GetTasks) (Utilities|Array|FindItem (Variables|Default|GetTasks) _task) _structout)
    (else
      (Development|PrintString "Не найдена задача!"))))

(event Custom|Overlaped
  (params (Actor :type Actor%20Object%20Reference) (Comp :type Primitive%20Component%20Object%20Reference))
  (bind _asbp_base_pickable (Utilities|Casting|CastToBP_BasePickable Actor))
  ;[1 1 1 1 12] Событие для того, чтобы несколько колизий в дочернем классе могли вызывать одинаковую логику
  (Utilities|IsAbletoUse
    (:Can%20Use
      (if (Utilities|DoesObjectImplementInterface Actor "/Game/Blueprints/Interfaces/I_PlugIn.I_PlugIn_C")
        (if (.TagAccepted (CallFunction|CheckforTag Actor))
          (Default|LetGofromPlayer _asbp_base_pickable Comp)
          (Variables|/Game/Blueprints/Props/Pickable/Classes/BP_BasePickable.BP_BasePickable_C|SetCanBePickedUp _asbp_base_pickable false)
          (CallFunction|Action Actor Comp))))))

(fn ConstructionScript)

(fn CheckforTag
  (params (Actor :type Actor%20Object%20Reference))
  (bind _acceptabletagsofoverlapactor (LocalVariables|GetAcceptableTagsOfOverlapActor))
  ;[1 1 1] Для каждого тега актера
  (for _array_element (Variables|Default|GetAcceptableTags)
    ;[1 1 1] Проверяем каждый тег  пересекающего актера
    (bind _array_element_2 (Utilities|Array|ForEachLoopwithBreak (Variables|/Script/Engine.Actor|GetTags Actor) :!label _label)
      (:LoopBody
        (if (Utilities|Name|Equal(Name) _array_element_2 _array_element)
          (Utilities|Array|Add (LocalVariables|GetAcceptableTagsOfOverlapActor) _array_element_2)
          (goto _label Break)))))
  (return (Utilities|Array|IsValidIndex _acceptabletagsofoverlapactor) _acceptabletagsofoverlapactor))

(fn Attach
  (params (Actor :type Actor%20Object%20Reference) (Component :type Scene%20Component%20Object%20Reference))
  (Transformation|AttachComponentToComponent Component (Variables|Default|GetAttachPoint) "None" "SnapToTarget" "SnapToTarget" "KeepWorld" true)
  (Variables|Default|SetIsUsing true))

(fn GetTaskbyTag
  (params (Array :type Array%20of%20Names))
  (bind _array_element (Utilities|Array|ForEachLoopwithBreak Array)
    (:LoopBody
      (bind _array_element_2 (Utilities|Array|ForEachLoopwithBreak (Variables|Default|GetTasks))
        (:LoopBody
          (if (not (.Done (Utilities|Struct|BreakS_LevelTasks _array_element_2)))
            (if (Utilities|Name|Equal(Name) (.ActorTag (Utilities|Struct|BreakS_LevelTasks _array_element_2)) _array_element)
              (return true _array_element_2))))))
    (:Completed
      (return false ""))))