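; BP_PlugPortBase is a base plug port that pickable objects snap into when they enter its Box trigger.
; On overlap, it casts the component's owner to BP_BasePickable and calls PlugGrabbedComponent on that pickable's Player.
; It then turns off physics on the component and attaches it to PlugPoint with snap-to-target rules.
; A successful attach stores the pickable as PluggedComponent.
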(event OnComponentBeginOverlap(Box)
  (params (OverlappedComponent :type Primitive%20Component%20Object%20Reference) (OtherActor :type Actor%20Object%20Reference) (OtherComp :type Primitive%20Component%20Object%20Reference) (OtherBodyIndex :type Integer) (bFromSweep :type Boolean) (SweepResult :type Hit%20Result%20Structure%20%28by%20ref%29))
  (CallFunction|PlugtoPort OtherComp))

(fn ConstructionScript)

(fn PlugtoPort
  (params (Component :type Primitive%20Component%20Object%20Reference))
  (Default|PlugGrabbedComponent (Variables|/Game/Blueprints/Calsses/Props/Pickable/Classes/BP_BasePickable.BP_BasePickable_C|GetPlayer (.AsBP%20Base%20Pickable (Utilities|Casting|CastToBP_BasePickable (Components|GetOwner Component)))) Component)
  (Physics|SetSimulatePhysics Component false)
  (bind _returnvalue (Transformation|AttachComponentToComponent Component (Variables|Components|GetPlugPoint) "None" "SnapToTarget" "SnapToTarget" "SnapToTarget" true))
  (if _returnvalue
    (Variables|Default|SetPluggedComponent (.AsBP%20Base%20Pickable (Utilities|Casting|CastToBP_BasePickable (Components|GetOwner Component))))))