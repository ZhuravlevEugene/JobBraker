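; Address flyer prop that the player interacts with to read a flyer listing addresses.
; Interaction creates the U_AdressFlyer widget, adds it to the viewport and changes the player input mode with the cursor shown.
; It then updates the level control's SpecialEvents, uniquely adding the found event and removing the not-found one, with a debug print when removal succeeds.
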(event EventBeginPlay
  (|CallParentFunction) ; This node is disabled and will not be called.\nDrag off pins to build functionality.
)

(event EventInteraction
  (bind _returnvalue (UserInterface|CreateWidget "/Game/Blueprints/UMG/SpecialWigets/Flyers/U_AdressFlyer.U_AdressFlyer_C" (.PlayerController (CallFunction|GetPlayer))))
  (UserInterface|Viewport|AddtoViewport _returnvalue 0)
  (CallFunction|ChangePlayerInputMode _returnvalue "NewEnumerator1" true)
  (bind _levelcontrol (CallFunction|GetLevelControl))
  (Utilities|Array|AddUnique (Variables|/Game/Blueprints/Calsses/LevelControl/LevelControls/LevelControlBase.LevelControlBase_C|GetSpecialEvents _levelcontrol) "AdressFliyerFound") ; Найден флайер с адресами
  (bind _returnvalue_2 (Utilities|Array|RemoveItem (Variables|/Game/Blueprints/Calsses/LevelControl/LevelControls/LevelControlBase.LevelControlBase_C|GetSpecialEvents _levelcontrol) "AdressFlyerNotFound"))
  (if _returnvalue_2
    (Development|PrintString "Flyer event removed")))

(fn ConstructionScript
  (|CallParentFunction))