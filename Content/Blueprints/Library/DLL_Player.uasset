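; DLL_Player is a library of helper functions for accessing the local player and switching its input mode.
; GetPlayer returns the first player's character cast to Player along with its controller, and stops if the cast fails.
; ChangePlayerInputMode uses that controller to apply game-only, UI-only or combined input, passing a widget to focus for the UI modes, then sets mouse cursor visibility.
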(fn GetPlayer
  (bind _asplayer (Utilities|Casting|CastToPlayer (Game|GetPlayerCharacter 0)))
  (return _asplayer (Game|GetPlayerController 0)))

(fn ChangePlayerInputMode
  (params (Widget :type Widget%20Object%20Reference) (InputMode :type E_DLL_InputModeType%20Enum :default "NewEnumerator0") (ShowCursor :type Boolean))
  (bind _playercontroller (CallFunction|GetPlayer))
  (switch Utilities|FlowControl|Switch|SwitchonE_DLL_InputModeType InputMode
    (:NewEnumerator0
      (Input|SetInputModeGameOnly _playercontroller))
    (:NewEnumerator1
      (Input|SetInputModeUIOnly _playercontroller Widget "DoNotLock"))
    (:NewEnumerator2
      (Input|SetInputModeGameandUI _playercontroller Widget "DoNotLock" true)))
  (Variables|/Script/Engine.PlayerController|SetbShowMouseCursor (Game|GetPlayerController 0) ShowCursor))