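; BP_BehaviorChecker is a level prop that tells the Player which named prop it is currently staying on.
; Entering MailCollision sets the player's StayingOn to this PropName and adds the checker to the player's OverlapedActors list.
; Leaving removes it and, if it was the current one, restores StayingOn from the last remaining entry or clears it, so overlapping zones fall back correctly.
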(event OnComponentBeginOverlap(MailCollision)
  (params (OverlappedComponent :type Primitive%20Component%20Object%20Reference) (OtherActor :type Actor%20Object%20Reference) (OtherComp :type Primitive%20Component%20Object%20Reference) (OtherBodyIndex :type Integer) (bFromSweep :type Boolean) (SweepResult :type Hit%20Result%20Structure%20%28by%20ref%29))
  (bind _asplayer (Utilities|Casting|CastToPlayer OtherActor))
  (Variables|/Game/Blueprints/Player.Player_C|SetStayingOn _asplayer (Variables|Default|GetPropName))
  (Utilities|Array|AddUnique (Variables|/Game/Blueprints/Player.Player_C|GetOverlapedActors (Variables|Default|GetPlayer)) self))

(event OnComponentEndOverlap(MailCollision)
  (params (OverlappedComponent :type Primitive%20Component%20Object%20Reference) (OtherActor :type Actor%20Object%20Reference) (OtherComp :type Primitive%20Component%20Object%20Reference) (OtherBodyIndex :type Integer))
  (bind _player (Variables|Default|GetPlayer))
  (bind _overlapedactors (Variables|/Game/Blueprints/Player.Player_C|GetOverlapedActors _player))
  (bind _returnvalue (Utilities|Array|LastIndex _overlapedactors))
  (bind _output (Utilities|Array|Get(acopy) _overlapedactors _returnvalue))
  (bind _asplayer (Utilities|Casting|CastToPlayer OtherActor))
  (if (Utilities|Enum|Equal(Enum) (Variables|Default|GetPropName) (Variables|/Game/Blueprints/Player.Player_C|GetStayingOn _asplayer))
    (Utilities|Array|RemoveItem (Variables|/Game/Blueprints/Player.Player_C|GetOverlapedActors (Variables|Default|GetPlayer)) self)
    (Variables|/Game/Blueprints/Player.Player_C|SetStayingOn _asplayer "")
    (Utilities|IsValid _output
      (:Is%20Valid
        (Variables|/Game/Blueprints/Player.Player_C|SetStayingOn _asplayer (Variables|BP_BehaviorChecker_C|GetPropName _output)))
      (:Is%20Not%20Valid
        (Variables|/Game/Blueprints/Player.Player_C|SetStayingOn _asplayer "")))
    (else
      (Utilities|Array|RemoveItem (Variables|/Game/Blueprints/Player.Player_C|GetOverlapedActors (Variables|Default|GetPlayer)) self))))

(event EventBeginPlay
  (Variables|Default|SetPlayer (.Player (CallFunction|GetPlayer))))

(fn ConstructionScript
  (|CallParentFunction))